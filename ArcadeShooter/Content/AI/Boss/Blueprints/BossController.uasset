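; AI controller for the boss that runs the Enemy_BT behavior tree and feeds it perception data.
; Perception updates pass each actor's last sensed stimuli to DoSenses, which identifies senses by array index, not class.
; The first stimulus sets CanSeePlayer; the second sets IsSearching and TargetLocation on the blackboard.
; OnKilled stops the brain logic, disables sight and turns off actor tick.
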(event `self.ReceiveBeginPlay`
  (`self.RunBehaviorTree` "/Game/AI/Enemy/Enemy_BT.Enemy_BT"))

(event `self.AIPerception.OnPerceptionUpdated`
  (params (UpdatedActors :type "Array of Actor Object Reference (by ref)"))
  (for _array_element UpdatedActors
    (bind _info (`AIPerceptionComponent.GetActorsPerception` (`self.AIPerception`) _array_element))
    (`self.DoSenses` (`.LastSensedStimuli` (break `ActorPerceptionBlueprintInfo` _info)))))

(event `/Game/FPSCharacter_BP/Weapon/Enemy_AI.On Killed`
  (`BrainComponent.StopLogic` (`self.BrainComponent`) "")
  (`AIPerceptionComponent.SetSenseEnabled` (`self.AIPerception`) "/Script/AIModule.AISense_Sight" false)
  (`self.SetActorTickEnabled` false))

(fn `DoSenses`
  (params (Array :type "Array of AIStimulus Structure"))
  (locals (`Local Senses` :type "AIStimulus Structure"))
  (bind (_local_senses_age _local_senses_expirationage _local_senses_strength _local_senses_stimuluslocation _local_senses_receiverlocation _local_senses_tag _local_senses_bsuccessfullysensed) (break `AIStimulus` (`local.Local Senses`)))
  (bind (_local_senses_age_2 _local_senses_expirationage_2 _local_senses_strength_2 _local_senses_stimuluslocation_2 _local_senses_receiverlocation_2 _local_senses_tag_2 _local_senses_bsuccessfullysensed_2) (break `AIStimulus` (`local.Local Senses`)))
  (for (_array_element _array_index) Array
    (set `local.Local Senses` _array_element)
    (switch `int` _array_index
      (:`0`
        (`BlackboardComponent.SetValueAsBool` (`AIBlueprintHelperLibrary.GetBlackboard` null) "CanSeePlayer" _local_senses_bsuccessfullysensed))
      (:`1`
        (`BlackboardComponent.SetValueAsBool` (`AIBlueprintHelperLibrary.GetBlackboard` null) "IsSearching" _local_senses_bsuccessfullysensed_2)
        (`BlackboardComponent.SetValueAsVector` (`AIBlueprintHelperLibrary.GetBlackboard` null) "TargetLocation" _local_senses_stimuluslocation_2)))))

(fn `UserConstructionScript`)