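; Boss enemy character that tracks its own health and fires projectiles from twin gun sockets.
; Damage lowers and prints health; at zero or below it sets the dead flag and blackboard IsDead key, notifies its controller and unpossesses.
; Attack raises an attacking flag, waits, spawns projectiles with gunshot sounds at both sockets using the mesh's rotation, then clears the flag after another delay.
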(event `self.ReceiveAnyDamage`
  (params (Damage :type "Float (single-precision)") (DamageType :type "DamageType Object Reference") (InstigatedBy :type "Controller Object Reference") (DamageCauser :type "Actor Object Reference"))
  (bind _returnvalue (`self.GetController`))
  (set `self.BossHealth` (- (`self.BossHealth`) Damage))
  (`KismetSystemLibrary.PrintString` (`KismetStringLibrary.Conv_DoubleToString` (`self.BossHealth`)))
  (if (<= (`self.BossHealth`) 0.0)
    (set `self.AmIDead` true)
    (`BlackboardComponent.SetValueAsBool` (`AIBlueprintHelperLibrary.GetBlackboard` null) "IsDead" true)
    (message `/Game/FPSCharacter_BP/Weapon/Enemy_AI.On Killed` _returnvalue)
    (`Controller.UnPossess` _returnvalue)))

(event `/Game/FPSCharacter_BP/Weapon/Enemy_AI.Attack`
  (bind _mesh (`self.Mesh`))
  (bind _returnvalue (`SceneComponent.GetSocketLocation` _mesh "LeftGun"))
  (bind _returnvalue_2 (`SceneComponent.GetSocketLocation` (`self.Mesh`) "RightGun"))
  (bind _returnvalue_3 (`SceneComponent.K2_GetComponentRotation` _mesh))
  (set `self.IsAttacking` true)
  (`KismetSystemLibrary.Delay` 1.0)
  (`|SpawnActorFromClass` "/Game/FPSCharacter_BP/Weapon/Projectile.Projectile_C" (`KismetMathLibrary.MakeTransform` _returnvalue _returnvalue_3) "Undefined" "OverrideRootScale" null null)
  (`|SpawnActorFromClass` "/Game/FPSCharacter_BP/Weapon/Projectile.Projectile_C" (`KismetMathLibrary.MakeTransform` _returnvalue_2 _returnvalue_3) "Undefined" "OverrideRootScale" null null)
  (`GameplayStatics.PlaySoundAtLocation` "/Game/Sounds/SFX/GunShot.GunShot" _returnvalue (struct) 1.0 1.0 0.0 null null null)
  (`GameplayStatics.PlaySoundAtLocation` "/Game/Sounds/SFX/GunShot.GunShot" _returnvalue_2 (struct) 1.0 1.0 0.0 null null null)
  (`KismetSystemLibrary.Delay` 2.0)
  (set `self.IsAttacking` false))

(fn `UserConstructionScript`)